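; Health component that tracks current health for its owner and signals player death.
; On BeginPlay it fills health to max and binds a handler to the OnHealthChanged dispatcher.
; The handler treats the incoming value as a signed delta, clamps the result between zero and max, and calls PlayerIsDead whenever health is at zero.
; GetHealth exposes the current value.
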(event `self.ReceiveBeginPlay`
  (set `self.CurrentHealth` (`self.MaxHealth`))
  (add `self.OnHealthChanged` (`|CreateDelegate` :!event `OnHealthChanged_Event`)))

(event `OnHealthChanged_Event` :!signature `self.OnHealthChanged`
  (params (Health :type "Float (double-precision)"))
  (bind _output_get (set `self.CurrentHealth` (`KismetMathLibrary.FClamp` (+ Health (`self.CurrentHealth`)) 0.0 (`self.MaxHealth`))))
  (if (<= _output_get 0.0)
    (`self.PlayerIsDead`)))

(fn `GetHealth`
  (returns (CurrentHealth :type "Float (double-precision)"))
  (return (`self.CurrentHealth`)))