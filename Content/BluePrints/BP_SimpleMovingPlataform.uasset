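; BP_SimpleMovingPlataform is an actor that moves a platform component between a Start and an End point.
; On BeginPlay it snaps the platform to Start, then plays a timeline.
; Each timeline update lerps the platform's world location between the two points using the PlataformSideMovement track, without sweeping.
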(event `self.ReceiveBeginPlay`
  (`SceneComponent.K2_SetWorldLocation` (`self.Plataform`) (`SceneComponent.K2_GetComponentLocation` (`self.Start`)) false false)
  (bind (_direction _plataformsidemovement) (`Timeline|Timeline`)
    (:`Update`
      (`SceneComponent.K2_SetWorldLocation` (`self.Plataform`) (`KismetMathLibrary.VLerp` (`SceneComponent.K2_GetComponentLocation` (`self.Start`)) (`SceneComponent.K2_GetComponentLocation` (`self.End`)) _plataformsidemovement) false false))))

(fn `UserConstructionScript`)