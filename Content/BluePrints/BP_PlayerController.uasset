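; Player controller that handles game input modes, the pause menu and the game-over screen.
; On BeginPlay it sets game-only input and binds to the player-death event on the third-person character's health component.
; The death handler shows the game-over widget with UI-only input and a visible cursor.
; The pause input toggles game pause, adding or removing the pause menu and switching input modes.
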(event `self.ReceiveBeginPlay`
  (`parent.ReceiveBeginPlay`)
  (bind _asbp_third_person_character (cast `/Game/ThirdPerson/Blueprints/BP_ThirdPersonCharacter` (`GameplayStatics.GetPlayerCharacter` 0)))
  (`WidgetBlueprintLibrary.SetInputMode_GameOnly` self)
  (set `self.bShowMouseCursor` false)
  (add `/Game/BluePrints/BP_HealthComponent.PlayerIsDead` (`/Game/ThirdPerson/Blueprints/BP_ThirdPersonCharacter.BP_HealthComponent` _asbp_third_person_character) (`|CreateDelegate` :!event `OnPlayerDied_Event`)))

(event `OnPlayerDied_Event`
  (bind _returnvalue (`|CreateWidget` "/Game/Widgets/W_GameOver.W_GameOver_C"))
  (`UserWidget.AddToViewport` _returnvalue 0)
  (`WidgetBlueprintLibrary.SetInputMode_UIOnlyEx` self _returnvalue)
  (set `self.bShowMouseCursor` true))

(event `EnhancedInput|/Game/BluePrints/CustomINputs/IA_PauseInput`
  (params (ActionValue :type Boolean) (ElapsedSeconds :type "Float (double-precision)") (TriggeredSeconds :type "Float (double-precision)") (InputAction :type "InputAction Object Reference" :default "/Game/BluePrints/CustomINputs/IA_PauseInput.IA_PauseInput"))
  (:`Triggered`
    (if (`GameplayStatics.IsGamePaused`)
      (`WidgetBlueprintLibrary.SetInputMode_GameOnly` self)
      (`GameplayStatics.SetGamePaused` false)
      (`Widget.RemoveFromParent` (`self.PauseHuD`))
      (else
        (bind _returnvalue (`|CreateWidget` "/Game/Widgets/W_PauseMenu.W_PauseMenu_C"))
        (bind _output_get (set `self.PauseHuD` _returnvalue))
        (`UserWidget.AddToViewport` _output_get 0)
        (`WidgetBlueprintLibrary.SetInputMode_UIOnlyEx` self null)
        (set `self.bShowMouseCursor` true)
        (`GameplayStatics.SetGamePaused` true)))))

(fn `UserConstructionScript`)